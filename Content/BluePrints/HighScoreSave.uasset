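; High score save Blueprint that holds an array of score structs and finds the best and worst entries in it.
; DetermineLowestScore and DetermineHighestScore each scan SaveStructs linearly, seeding from the first element and replacing it only on a strictly lower or higher Score, so ties keep the earliest entry.
; Each returns the winning struct with its index, with no guard for an empty array.
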(fn DetermineLowestScore
  (for (_array_element _array_index) (Variables|Default|GetSaveStructs)
    (if (== _array_index 0)
      (LocalVariables|SetLowestScore (.score _array_element))
      (LocalVariables|SetLowestIndex _array_index)
      (elif (< (.score _array_element) (LocalVariables|GetLowestScore))
        (LocalVariables|SetLowestScore (.score _array_element))
        (LocalVariables|SetLowestIndex _array_index))))
  (return (Utilities|Array|Get(acopy) (Variables|Default|GetSaveStructs) (LocalVariables|GetLowestIndex)) (LocalVariables|GetLowestIndex)))

(fn DetermineHighestScore
  (for (_array_element _array_index) (Variables|Default|GetSaveStructs)
    (if (== _array_index 0)
      (LocalVariables|SetHighestScore (.score _array_element))
      (LocalVariables|SetHighestIndex _array_index)
      (elif (> (.score _array_element) (LocalVariables|GetHighestScore))
        (LocalVariables|SetHighestScore (.score _array_element))
        (LocalVariables|SetHighestIndex _array_index))))
  (return (Utilities|Array|Get(acopy) (Variables|Default|GetSaveStructs) (LocalVariables|GetHighestIndex)) (LocalVariables|GetHighestIndex)))