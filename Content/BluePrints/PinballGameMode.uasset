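; Pinball game mode that runs the ball lifecycle, multiplied scoring and end-of-game high score check.
; Spawns BP_Ball at the plunger and respawns it on destruction until BallsRemaining runs out.
; EndGame lazily loads or creates a cached HighScoreSave, showing HighScoreEntry if it holds three or fewer entries.
; Beating the lowest score in a fuller list leads nowhere, and CreateMainMenu also opens HighScoreEntry.
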(event Custom|SpawnBall
  (bind _outactors (Actor|GetAllActorsOfClass "/Game/BluePrints/BP_Plunger.BP_Plunger_C"))
  (bind _returnvalue (Game|SpawnActorfromClass "/Game/BluePrints/BP_Ball.BP_Ball_C" (Math|Transform|MakeTransform (Default|GetBallSpawnLocation (Utilities|Array|Get(acopy) _outactors)) "0, 0, 0" "1,1,1") "Undefined" 0 0))
  (Game|BindEventtoOnDestroyed _returnvalue (delegate Custom|onBallDestroy)))

(event Custom|CreateMainMenu
  (bind _returnvalue (Game|GetPlayerController 0))
  (bind _aspinball_player_controller (Utilities|Casting|CastToPinballPlayerController _returnvalue))
  (Viewport|RemoveAllWidgets)
  (bind _returnvalue_2 (UserInterface|CreateWidget "/Game/BluePrints/HighScoreEntry.HighScoreEntry_C" _aspinball_player_controller))
  (UserInterface|Viewport|AddtoViewport _returnvalue_2 0)
  (Variables|/Script/Engine.PlayerController|SetbShowMouseCursor _aspinball_player_controller true))

(event Custom|EndGame
  (bind _currentsaveobject (CallFunction|GetSaveGameData))
  (if (<= (Utilities|Array|Length (Variables|/Game/BluePrints/HighScoreSave.HighScoreSave_C|GetSaveStructs _currentsaveobject)) 3)
    (CallFunction|CreateHighScoresList)
    (else
      (bind _lowestscorestruct (Default|DetermineLowestScore _currentsaveobject))
      (if (< (.score _lowestscorestruct) (Variables|Default|GetScore))
        _))))

(event Custom|onBallDestroy
  (params (DestroyedActor :type Actor%20Object%20Reference))
  (if (> (Variables|Default|GetBallsRemaining) 0)
    (CallFunction|SpawnBall)
    (Math|Integer|DecrementInt (Variables|Default|GetBallsRemaining))
    (else
      (CallFunction|EndGame))))

(event Custom|CreateHighScoresList
  (bind _returnvalue (Game|GetPlayerController 0))
  (bind _aspinball_player_controller (Utilities|Casting|CastToPinballPlayerController _returnvalue))
  (bind _returnvalue_2 (UserInterface|CreateWidget "/Game/BluePrints/HighScoreEntry.HighScoreEntry_C" _aspinball_player_controller))
  (UserInterface|Viewport|AddtoViewport _returnvalue_2 0)
  (Variables|/Script/Engine.PlayerController|SetbShowMouseCursor _aspinball_player_controller true))

(event EventBeginPlay
  (CallFunction|SpawnBall))

(event EventTick
  (params (DeltaSeconds :type Float%20%28single-precision%29)))

(fn ConstructionScript)

(fn AddScore
  (params (PointsToAdd :type Float%20%28single-precision%29))
  (bind _output_get (Variables|Default|SetScore (+ (* PointsToAdd (Variables|Default|GetMultiplier)) (Variables|Default|GetScore))))
  (return _output_get))

(fn GetSaveGameData
  (bind _currentsaveobject (Variables|Default|GetCurrentSaveObject)
    (:then
      (return _currentsaveobject))
    (:else
      (bind _returnvalue (SaveGame|DoesSaveGameExist (Variables|Default|GetHighScoreSaveName)))
      (if _returnvalue
        (bind _returnvalue_2 (SaveGame|LoadGamefromSlot (Variables|Default|GetHighScoreSaveName)))
        (bind _ashigh_score_save (Utilities|Casting|CastToHighScoreSave _returnvalue_2)
          (:then
            (Default|SortSaveData _ashigh_score_save)
            (bind _output_get (Variables|Default|SetCurrentSaveObject _ashigh_score_save))
            (return _output_get))
          (:CastFailed
            _))
        (else
          (bind _returnvalue_3 (SaveGame|CreateSaveGameObject "/Game/BluePrints/HighScoreSave.HighScoreSave_C"))
          (bind _ashigh_score_save_2 (Utilities|Casting|CastToHighScoreSave _returnvalue_3)
            (:then
              (bind _output_get_2 (Variables|Default|SetCurrentSaveObject _ashigh_score_save_2))
              (return _output_get_2))
            (:CastFailed
              _))))
      (return 0))))